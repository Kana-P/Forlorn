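; Kurayami is a player character Blueprint with world-axis movement, a stamina-limited sprint and death-driven level changes.
; Sprinting raises walk speed and drains stamina on a looping timer while moving; Tick regenerates it after a delay, and BeginPlay adds the StaminaBar widget.
; P zeroes Health and calls Level1, which counts deaths and streak and opens the next map.
; Level2/Level3 branches are unwired; ToBadEnd is never called here.
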(event Custom|Stamina%20Drain
  ;[1 1 1] Drain Stamina
  (if (> (Math|Vector|VectorLength (Variables|/Script/Engine.MovementComponent|GetVelocity (Variables|Character|GetCharacterMovement))) 0.0)
    (Variables|Default|SetStamina (Math|Float|Max(Float) (- (Variables|Default|GetStamina) 0.1) 0.0))
    (if (not (> (Variables|Default|GetStamina) 0.0))
      (Variables|/Script/Engine.CharacterMovementComponent|SetMaxWalkSpeed (Variables|Character|GetCharacterMovement) 5e+02)
      (Utilities|Time|ClearTimerbyFunctionName 0 "Stamina Drain")
      (Variables|Default|SetisSprinting false))))

(event EventTick
  (params (DeltaSeconds :type Float%20%28single-precision%29))
  ;[1 1 1] Stamina Regen
  (if (not (Variables|Default|GetisSprinting))
    (Utilities|FlowControl|Delay 1.0)
    (Variables|Default|SetStamina (Math|Float|Min(Float) (+ (Variables|Default|GetStamina) (Variables|Default|GetStaminaRate)) 1.0))))

(event EventBeginPlay
  (bind _returnvalue (UserInterface|CreateWidget "/Game/ForlornAssets/HUD/StaminaBar.StaminaBar_C"))
  (UserInterface|Viewport|AddtoViewport _returnvalue 0))

(event Input|ActionEvents|InputActionSprint
  (params (Key :type Key%20Structure :default "None"))
  (bind _charactermovement (Variables|Character|GetCharacterMovement))
  ;[1 1 1] Sprint
  (:Pressed
    (if (>= (Variables|Default|GetStamina) 0.0)
      (Variables|/Script/Engine.CharacterMovementComponent|SetMaxWalkSpeed _charactermovement 8e+02)
      (bind _output_get (Variables|Default|SetisSprinting true))
      (Utilities|Time|SetTimerbyFunctionName 0 "Stamina Drain" 0.5 _output_get)))
  (:Released
    (Variables|/Script/Engine.CharacterMovementComponent|SetMaxWalkSpeed _charactermovement 5e+02)
    (Utilities|Time|ClearTimerbyFunctionName 0 "Stamina Drain")
    (Variables|Default|SetisSprinting false)))

(event Input|AxisEvents|InputAxisMoveForward
  (params (AxisValue :type Float%20%28single-precision%29))
  ;[1 1 1] Basic Movement
  (Pawn|Input|AddMovementInput "90.000000, 0, 0" AxisValue false))

(event Input|AxisEvents|InputAxisMoveRight
  (params (AxisValue :type Float%20%28single-precision%29))
  ;[1 1 1] Basic Movement
  (Pawn|Input|AddMovementInput "0.000000,90.000000, 0" AxisValue false))

(event Input|KeyboardEvents|P
  (params (Key :type Key%20Structure :default "None"))
  (:Pressed
    (Variables|Default|SetHealth 0.0)
    (if (== (Variables|Default|GetCurrentLevel) 1)
      (CallFunction|Level1))))

(fn ConstructionScript)

(fn Level1
  (if (== (Variables|Default|GetHealth) 0.0)
    (Variables|Default|SetHealth 1.0)
    (Variables|Default|SetDeathCount (+ (Variables|Default|GetDeathCount) 1))
    (Variables|Default|SetDeathStreak (+ (Variables|Default|GetDeathStreak) 1))
    (Variables|Default|SetCurrentLevel (+ (Variables|Default|GetCurrentLevel) 1))
    (Game|OpenLevel(byName) "test2")))

(fn Level2
  (if (== (Variables|Default|GetHealth) 0.0)
    (Variables|Default|SetHealth 1.0)
    (Variables|Default|SetDeathCount (+ (Variables|Default|GetDeathCount) 1))
    (if (> (Variables|Default|GetDeathStreak) 0)
      (Variables|Default|SetDeathStreak (+ (Variables|Default|GetDeathStreak) 1))
      (else
        (Variables|Default|SetDeathStreak 0)))
    (Variables|Default|SetCurrentLevel (+ (Variables|Default|GetCurrentLevel) 1))
    (Game|OpenLevel(byName) "test3")))

(fn Level3
  (if (== (Variables|Default|GetHealth) 0.0)
    (Variables|Default|SetHealth 1.0)
    (Variables|Default|SetDeathCount (+ (Variables|Default|GetDeathCount) 1))
    (if (> (Variables|Default|GetDeathStreak) 0)
      (Variables|Default|SetDeathStreak (+ (Variables|Default|GetDeathStreak) 1))
      (else
        (Variables|Default|SetDeathStreak 0)))
    (Variables|Default|SetCurrentLevel (+ (Variables|Default|GetCurrentLevel) 1))
    (Game|OpenLevel(byName) "Test1")))

(fn Level4)

(fn Level5)

(fn ToBadEnd
  (if (== (Variables|Default|GetDeathStreak) 3)
    (Game|OpenLevel(byName) "Badend")))